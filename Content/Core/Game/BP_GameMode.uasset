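; Game mode that spawns both players' rubber teams from the game instance at BeginPlay.
; P1's team classes spawn at start "P1"; player controller 0 possesses each in turn and blends its view to a level CameraActor.
; P2's team only sets the spawn count: each pawn is a BP_Rubber_Base at start "P2", passed to the same controller via SetupP2Pawn.
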(event EventBeginPlay
  (bind _returnvalue (Game|GetPlayerController 0))
  (Utilities|FlowControl|Sequence
    (:then_0
      (bind _asbp_game_instance (Utilities|Casting|CastToBP_GameInstance (Game|GetGameInstance)))
      (for _array_element (Variables|/Game/Core/Game/BP_GameInstance.BP_GameInstance_C|GetP1_RubberTeam _asbp_game_instance)
        (bind _returnvalue_2 (Game|SpawnActorfromClass _array_element (Transformation|GetActorTransform (Class|GameModeBase|FindPlayerStart 0 "P1")) "Undefined" "MultiplyWithRoot" 0 0))
        (bind _asbp_player_controller (Utilities|Casting|CastToBP_PlayerController _returnvalue))
        (Pawn|Possess _asbp_player_controller _returnvalue_2)
        (bind _returnvalue_3 (Actor|GetActorOfClass "/Script/Engine.CameraActor"))
        (Game|Player|SetViewTargetwithBlend (Game|GetPlayerController 0) _returnvalue_3 1.0 "VTBlend_Linear" 0.0 false)))
    (:then_1
      (bind _asbp_game_instance_2 (Utilities|Casting|CastToBP_GameInstance (Game|GetGameInstance)))
      (for _array_element_2 (Variables|/Game/Core/Game/BP_GameInstance.BP_GameInstance_C|GetP2_RubberTeam _asbp_game_instance_2)
        (bind _returnvalue_4 (Game|SpawnActorfromClass "/Game/Core/Player/BP_Rubber_Base.BP_Rubber_Base_C" (Transformation|GetActorTransform (Class|GameModeBase|FindPlayerStart 0 "P2")) "Undefined" "MultiplyWithRoot" 0 0))
        (bind _asbp_player_controller_2 (Utilities|Casting|CastToBP_PlayerController _returnvalue))
        (Default|SetupP2Pawn _asbp_player_controller_2 _returnvalue_4)))))

(fn ConstructionScript)