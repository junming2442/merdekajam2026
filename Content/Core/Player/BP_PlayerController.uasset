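; Player controller for a local two-player, turn-based game in which one controller drives both rubber pawns.
; It adds both players' input mappings on possess, stores P1 from the controlled pawn and receives P2 through SetupP2Pawn.
; Move input reaches only the current player's pawn, with DoOnce-gated charge sounds and a scoreboard turn image update on release.
; HandlePlayerMoved, not triggered by live wiring here, swaps the active player ID and pawn turns.
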(event Custom|SetupP2Pawn
  (params (Pawn :type Actor%20Object%20Reference))
  (bind _asbp_rubber_base (Utilities|Casting|CastToBP_Rubber_Base Pawn))
  (bind _output_get (Variables|Default|SetP2_Pawn _asbp_rubber_base))
  (Default|Setup _output_get)
  (Default|DismissTurn _output_get))

(event Custom|HandlePlayerMoved
  (Utilities|FlowControl|Delay 0.0)
  (switch int (Variables|Default|GetCurrentRoundPlayerID)
    (:0
      (Default|IsYouMotherFkerTurn (Variables|Default|GetP2_Pawn))
      (Variables|Default|SetCurrentRoundPlayerID 1)
      (Default|DismissTurn (Variables|Default|GetP1_Pawn)))
    (:1
      (Default|IsYouMotherFkerTurn (Variables|Default|GetP1_Pawn))
      (Variables|Default|SetCurrentRoundPlayerID 0)
      (Default|DismissTurn (Variables|Default|GetP2_Pawn)))))

(event Custom|Reset%20Charging%20Sound%201
  ;[0.15 0.15 0.15 0.5] Move
  (Utilities|FlowControl|DoOnce false) ; enters at Reset
)

(event Custom|Reset%20Charging%20Sound%202
  ;[0.15 0.15 0.15 0.5] Move
  (Utilities|FlowControl|DoOnce false) ; enters at Reset
)

(event Input|EnhancedActionEvents|EnhancedInputActionIA_Move_P1
  (params (ActionValue :type Vector%202D%20Structure) (ElapsedSeconds :type Float%20%28double-precision%29) (TriggeredSeconds :type Float%20%28double-precision%29) (InputAction :type Input%20Action%20Object%20Reference :default "/Game/Core/Input/IA_Move_P1.IA_Move_P1"))
  ;[0.15 0.15 0.15 0.5] Move
  (:Triggered
    (if (== (Variables|Default|GetCurrentRoundPlayerID) 0)
      (Utilities|FlowControl|DoOnce false
        (:Completed
          (bind _returnvalue (Audio|SpawnSound2D "/Game/Sound/Sound_Effect/BuildUp-Charge.BuildUp-Charge" 1.0 1.0 0.0 0 false false))
          (Variables|Default|SetChargin%20Sound _returnvalue)
          (if (== (Variables|Default|GetCurrentRoundPlayerID) 0)
            (Default|Move (Variables|Default|GetP1_Pawn) ActionValue :!label _label))))))
  (:Completed
    (if (== (Variables|Default|GetCurrentRoundPlayerID) 0)
      (CallFunction|ResetChargingSound1)
      (Appearance|SetBrushfromTexture (Variables|/Game/Core/UI/WBP_Scoreboard.WBP_Scoreboard_C|GetWhoTurn? (Variables|/Game/Core/UI/BP_HUD.BP_HUD_C|GetScoreboardWidget (Variables|Default|GetBP_Hud))) "/Game/Ui/Ui_Image/player_2_turn.player_2_turn" false)
      (Audio|Components|Audio|Stop (Variables|Default|GetChargin%20Sound))
      (if (== (Variables|Default|GetCurrentRoundPlayerID) 0)
        (goto _label)))))

(event Input|EnhancedActionEvents|EnhancedInputActionIA_Move_P2
  (params (ActionValue :type Vector%202D%20Structure) (ElapsedSeconds :type Float%20%28double-precision%29) (TriggeredSeconds :type Float%20%28double-precision%29) (InputAction :type Input%20Action%20Object%20Reference :default "/Game/Core/Input/IA_Move_P2.IA_Move_P2"))
  ;[0.15 0.15 0.15 0.5] Move
  (:Triggered
    (if (== (Variables|Default|GetCurrentRoundPlayerID) 1)
      (Utilities|FlowControl|DoOnce false
        (:Completed
          (bind _returnvalue (Audio|SpawnSound2D "/Game/Sound/Sound_Effect/BuildUp-Charge.BuildUp-Charge" 1.0 1.0 0.0 0 false false))
          (Variables|Default|SetChargin%20Sound _returnvalue)
          (if (== (Variables|Default|GetCurrentRoundPlayerID) 1)
            (Default|Move (Variables|Default|GetP2_Pawn) ActionValue :!label _label))))))
  (:Completed
    (if (== (Variables|Default|GetCurrentRoundPlayerID) 1)
      (CallFunction|ResetChargingSound2)
      (Appearance|SetBrushfromTexture (Variables|/Game/Core/UI/WBP_Scoreboard.WBP_Scoreboard_C|GetWhoTurn? (Variables|/Game/Core/UI/BP_HUD.BP_HUD_C|GetScoreboardWidget (Variables|Default|GetBP_Hud))) "/Game/Ui/Ui_Image/player_1_turn.player_1_turn" false)
      (Audio|Components|Audio|Stop (Variables|Default|GetChargin%20Sound))
      (if (== (Variables|Default|GetCurrentRoundPlayerID) 1)
        (goto _label)))))

(event EventBeginPlay
  (bind _asbp_game_mode (Utilities|Casting|CastToBP_GameMode (Game|GetGameMode)))
  (Variables|Default|SetGameModeRef _asbp_game_mode)
  (bind _asbp_hud (Utilities|Casting|CastToBP_HUD (HUD|GetHUD)))
  (Variables|Default|SetBP_Hud _asbp_hud)
  (bind _asbp_rubber_base (Utilities|Casting|CastToBP_Rubber_Base (Game|Player|GetPlayerPawn 0)))
  (Variables|Default|SetBP_RubberBase _asbp_rubber_base))

(event EventPossess
  (params (PossessedPawn :type Pawn%20Object%20Reference))
  (bind _returnvalue (PlayerController|LocalPlayerSubsystems|GetEnhancedInputLocalPlayerSubsystem))
  (Utilities|FlowControl|Sequence
    (:then_0
      (Input|AddMappingContext _returnvalue "/Game/Core/Input/IMC_P1.IMC_P1" 0 "(bIgnoreAllPressedKeysUntilRelease=True,bForceImmediately=False,bNotifyUserSettings=False)")
      (Input|AddMappingContext _returnvalue "/Game/Core/Input/IMC_P2.IMC_P2" 0 "(bIgnoreAllPressedKeysUntilRelease=True,bForceImmediately=False,bNotifyUserSettings=False)"))
    (:then_1
      (bind _asbp_rubber_base (Utilities|Casting|CastToBP_Rubber_Base (Pawn|GetControlledPawn)))
      (bind _output_get (Variables|Default|SetP1_Pawn _asbp_rubber_base))
      (Default|Setup _output_get))))

(fn ConstructionScript)