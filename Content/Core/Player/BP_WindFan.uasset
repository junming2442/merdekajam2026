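; BP_WindFan is a fan actor that blows tagged physics objects within its wind zone.
; Each tick it loops over actors overlapping WindZone and applies WindForce, in the fan's local space, as acceleration to the static mesh component of those tagged "Blowable".
; FanBlades rotation runs inside the same loop, so the blades spin only while actors overlap the zone, faster with each additional one.
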(event Collision|EventActorBeginOverlap
  (params (OtherActor :type Actor%20Object%20Reference)))

(event EventTick
  (params (DeltaSeconds :type Float%20%28single-precision%29))
  (for _array_element (Collision|GetOverlappingActors (Variables|Default|GetWindZone) 0 :!class /Script/Engine.PrimitiveComponent)
    (Utilities|FlowControl|Sequence
      (:then_0
        (if (Actor|ActorHasTag _array_element "Blowable")
          (Physics|AddForce (Actor|GetComponentbyClass _array_element "/Script/Engine.StaticMeshComponent") (Math|Transform|TransformDirection (Transformation|GetActorTransform) (Variables|Default|GetWindForce)) "None" true)))
      (:then_1
        (Transformation|AddLocalRotation (Variables|Default|GetFanBlades) (Math|Rotator|MakeRotator (* DeltaSeconds 3e+02) 0.0 0.0) false false)))))

(event EventBeginPlay)

(fn ConstructionScript)