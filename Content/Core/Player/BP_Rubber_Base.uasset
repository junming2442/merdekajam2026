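; Base physics pawn for a turn-based rubber-flicking game, with mesh and tuning taken from RubberDetails.
; Holding stick input charges a HUD bar; release applies scaled linear and flip impulses, then disables input and notifies controller and GameMode.
; Resting higher on another rubber reports a win, and touching a kill zone reports death, both DoOnce-gated until round reset.
; Cannon hits apply radial impulses.
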(event OnComponentBeginOverlap(StaticMesh)
  (params (OverlappedComponent :type Primitive%20Component%20Object%20Reference) (OtherActor :type Actor%20Object%20Reference) (OtherComp :type Primitive%20Component%20Object%20Reference) (OtherBodyIndex :type Integer) (bFromSweep :type Boolean) (SweepResult :type Hit%20Result%20Structure%20%28by%20ref%29))
  ;[0.15 0.15 0.15 0.5] Check Dead
  (Utilities|Casting|CastToBP_KillZone OtherActor)
  (Utilities|FlowControl|DoOnce false
    (:Completed
      (Default|Died (Variables|Default|GetGameModeRef) self))))

(event OnComponentHit(StaticMesh)
  (params (HitComponent :type Primitive%20Component%20Object%20Reference) (OtherActor :type Actor%20Object%20Reference) (OtherComp :type Primitive%20Component%20Object%20Reference) (NormalImpulse :type Vector :default "0, 0, 0") (Hit :type Hit%20Result%20Structure%20%28by%20ref%29))
  ;[0.15 0.15 0.15 0.5] Check Overlap
  (bind _returnvalue (Physics|GetPhysicsLinearVelocity (Variables|Default|GetStaticMesh) "None"))
  (if (<= (Math|Vector|VectorLength _returnvalue) 0.0)
    (bind _asbp_rubber_base (Utilities|Casting|CastToBP_Rubber_Base OtherActor))
    (if (>= (- (CallFunction|GetAbsoluteHeight self) (CallFunction|GetAbsoluteHeight _asbp_rubber_base)) 0.2)
      (Utilities|FlowControl|DoOnce false
        (:Completed
          (Default|Win (Variables|Default|GetGameModeRef) self))))))

(event Custom|Move
  (params (Input :type Vector%202D%20Structure))
  (bind _returnvalue (Class|KismetMathLibrary|NormalSafe2D Input 0.0))
  (bind (_x _y) (Math|Vector2D|BreakVector2D _returnvalue))
  ;[0.15 0.15 0.15 0.5] Move
  (if (> (Math|Vector2D|Vector2DLength Input) 0.7)
    (Variables|Default|SetIsCharging true)
    (Utilities|FlowControl|Delay 0.05)
    (Variables|Default|SetLastMoveDirection (Math|Vector|MakeVector _y _x (.LiftPower (Utilities|Struct|BreakF_RubberDetails (Variables|Default|GetRubberDetails)))))
    (elif (Variables|Default|GetIsCharging)
      (CallFunction|Launch))))

(event Custom|Launch
  ;[0.15 0.15 0.15 0.5] Move
  (Audio|PlaySound2D "/Game/Sound/Sound_Effect/boings1.boings1" 4.0 1.0 0.0 0 0)
  (Variables|Default|SetIsCharging false)
  (bind _launchpower (CallFunction|GetLaunchPower))
  (Physics|AddImpulse (Variables|Default|GetStaticMesh) _launchpower "None" true)
  (bind _flippower (CallFunction|GetFlipPower))
  (Class|PrimitiveComponent|AddAngularImpulseinDegrees (Variables|Default|GetStaticMesh) _flippower "None" true)
  (Variables|Default|SetCurrentCharge 0.0)
  (Progress|SetPercent (Variables|/Game/Core/UI/WBP_HUD.WBP_HUD_C|GetProgressBar_Charge (Variables|Default|GetDebugWidget)) 0.0)
  ;;[0.15 0.15 0.15 0.5] Cooldown
  (Default|DisablePlayerInput (Variables|Default|GetGameModeRef))
  (bind _asbp_player_controller (Utilities|Casting|CastToBP_PlayerController (Game|GetPlayerController 0)))
  (Default|HandlePlayerMoved _asbp_player_controller)
  (Default|CheckAnyMoving (Variables|Default|GetGameModeRef)))

(event Custom|HandleResetRound
  ;[0.15 0.15 0.15 0.5] Check Overlap
  (Utilities|FlowControl|Sequence
    (:then_0
      (Utilities|FlowControl|DoOnce false) ; enters at Reset
    )
    (:then_1
      ;[0.15 0.15 0.15 0.5] Check Dead
      (Utilities|FlowControl|DoOnce false) ; enters at Reset
    )))

(event Custom|Setup
  ;[0.15 0.15 0.15 0.5] Setup
  (bind _aswbp_hud (Utilities|Casting|CastToWBP_HUD (UserInterface|GetUserWidgetObject (Variables|Default|GetWidget))))
  (Variables|Default|SetDebugWidget _aswbp_hud)
  (bind _asbp_game_mode (Utilities|Casting|CastToBP_GameMode (Game|GetGameMode)))
  (bind _output_get (Variables|Default|SetGameModeRef _asbp_game_mode))
  (EventDispatchers|BindEventtoOnResetRound _output_get (EventDispatchers|CreateEvent :!event Custom|HandleResetRound)))

(event Custom|HitByCannon
  (params (Location :type Vector))
  (Physics|AddRadialImpulse (Variables|Default|GetStaticMesh) (- Location "0.000000,0.000000,100.000000") 3e+02 6e+02 "RIF_Constant" true))

(event Custom|Dismiss%20Turn
  (Widget|SetVisibility (Variables|/Game/Core/UI/WBP_HUD.WBP_HUD_C|GetProgressBar_Charge (Variables|Default|GetDebugWidget)) "Hidden"))

(event Custom|Is%20You%20Mother%20Fker%20Turn
  (Widget|SetVisibility (Variables|/Game/Core/UI/WBP_HUD.WBP_HUD_C|GetProgressBar_Charge (Variables|Default|GetDebugWidget)) "Visible"))

(event EventTick
  (params (DeltaSeconds :type Float%20%28single-precision%29))
  ;[0.15 0.15 0.15 0.5] Tick
  (Transformation|SetWorldLocation (Variables|Default|GetWidget) (+ (Transformation|GetWorldLocation (Variables|Default|GetStaticMesh)) "0.000000,0.000000,100.000000") false false)
  (if (Variables|Default|GetIsCharging)
    (bind _output_get (Variables|Default|SetCurrentCharge (Math|Float|Clamp(Float) (+ (Variables|Default|GetCurrentCharge) (* (Utilities|Time|GetWorldDeltaSeconds) (.ChargeRate (Utilities|Struct|BreakF_RubberDetails (Variables|Default|GetRubberDetails))))))))
    (Progress|SetPercent (Variables|/Game/Core/UI/WBP_HUD.WBP_HUD_C|GetProgressBar_Charge (Variables|Default|GetDebugWidget)) _output_get)))

(event Input|KeyboardEvents|P
  (params (Key :type Key%20Structure :default "None"))
  (:Pressed
    (Default|ResetRound (Variables|Default|GetGameModeRef))))

(fn ConstructionScript
  (bind _staticmesh (Variables|Default|GetStaticMesh))
  (bind _rubberdetails (Variables|Default|GetRubberDetails))
  (bind (_icon _displayname _mesh _massscale) (Utilities|Struct|BreakF_RubberDetails _rubberdetails))
  (Components|StaticMesh|SetStaticMesh _staticmesh _mesh)
  (Class|PrimitiveComponent|SetMassScale _staticmesh "None" _massscale))

(fn GetFlipPower
  (bind _lastmovedirection (Variables|Default|GetLastMoveDirection))
  (bind (_x _y) (Math|Vector|BreakVector _lastmovedirection))
  (return (* (Math|Vector|MakeVector (* _y -1.0) _x 0.0) (* (Variables|Default|GetCurrentCharge) (.BaseFlipPower (Utilities|Struct|BreakF_RubberDetails (Variables|Default|GetRubberDetails)))))))

(fn GetLaunchPower
  (bind _rubberdetails (Variables|Default|GetRubberDetails))
  (bind (_icon _massscale _baseimpulse) (Utilities|Struct|BreakF_RubberDetails _rubberdetails))
  (return (* (Variables|Default|GetLastMoveDirection) (/ (* (Variables|Default|GetCurrentCharge) _baseimpulse) _massscale))))

(fn GetAbsoluteHeight
  (params (RubberActor :type BP%20Rubber%20Base%20Object%20Reference))
  (bind _staticmesh (Variables|BP_Rubber_Base_C|GetStaticMesh RubberActor))
  (bind (_min _max) (Components|StaticMesh|GetLocalBounds _staticmesh))
  (return (/ (.z (Transformation|GetActorLocation RubberActor)) (- (.Z (Math|Vector|BreakVector _max)) (.Z (Math|Vector|BreakVector _min))))))