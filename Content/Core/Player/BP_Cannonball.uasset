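; BP_Cannonball is a cannonball projectile that delivers an area impact to rubber actors when it hits something other than a BP_Cannon.
; On mesh hit, a multi sphere trace at the impact point finds nearby actors and calls HitByCannon on each BP_Rubber_Base hit.
; The bomb sound and self-destruction sit inside the trace loop, so they run per hit result and not at all when the trace returns nothing.
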(event OnComponentHit(StaticMesh)
  (params (HitComponent :type Primitive%20Component%20Object%20Reference) (OtherActor :type Actor%20Object%20Reference) (OtherComp :type Primitive%20Component%20Object%20Reference) (NormalImpulse :type Vector :default "0, 0, 0") (Hit :type Hit%20Result%20Structure%20%28by%20ref%29))
  (bind _location (Collision|BreakHitResult Hit))
  (Utilities|Casting|CastToBP_Cannon OtherActor
    (:CastFailed
      (bind _outhits (Collision|MultiSphereTraceByChannel _location _location 3e+02 "TraceTypeQuery1" false (Utilities|Array|MakeArray self) "None"))
      (for _array_element _outhits
        (bind _asbp_rubber_base (Utilities|Casting|CastToBP_Rubber_Base (.HitActor (Collision|BreakHitResult _array_element)))
          (:then
            (Default|HitbyCannon _asbp_rubber_base (.Location (Collision|BreakHitResult _array_element))))
          (:CastFailed
            _))
        (Audio|PlaySound2D "/Game/Sound/Sound_Effect/Cannon_Bomb.Cannon_Bomb" 0.05 1.0 0.0 0 0)
        (Actor|DestroyActor)))))

(fn ConstructionScript)