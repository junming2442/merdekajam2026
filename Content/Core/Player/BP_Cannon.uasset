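; BP_Cannon is a cannon that lobs physics cannonballs at areas around BP_Rubber_Base actors.
; It binds to the game mode's OnFinishMoving event after a one-tick delay, with a weighted random chance of firing each time.
; A shot plays a sound, picks a random point near a random rubber actor and yaws the mesh toward it.
; SuggestProjectileVelocityCustomArc supplies the launch velocity for the cannonball spawned at the arrow.
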(event Custom|FireCannon
  (bind _cannonmesh (Variables|Default|GetCannonMesh))
  (bind _arrow (Variables|Default|GetArrow))
  (bind _returnvalue (Transformation|GetWorldLocation _arrow))
  (if (Math|Random|RandomBoolwithWeight 0.6)
    (Audio|PlaySound2D "/Game/Sound/Sound_Effect/Cannon_Shoot.Cannon_Shoot" 0.5 1.0 0.5 0 0)
    (bind _outactors (Actor|GetAllActorsOfClass "/Game/Core/Player/BP_Rubber_Base.BP_Rubber_Base_C"))
    (if (Utilities|Array|IsNotEmpty _outactors)
      (Variables|Default|SetRandomLocation (Math|Random|RandomPointinBoundingBox (Transformation|GetActorLocation (.OutItem (Utilities|Array|Random _outactors))) "200.000000,200.000000,0.000000"))
      (Transformation|SetWorldRotation _cannonmesh (Math|Rotator|MakeRotator 0.0 0.0 (.yaw (Math|Rotator|FindLookatRotation (Transformation|GetWorldLocation _cannonmesh) (Variables|Default|GetRandomLocation)))) false false)
      (bind _outlaunchvelocity (Game|SuggestProjectileVelocityCustomArc _returnvalue (Variables|Default|GetRandomLocation) 0.0 0.5))
      (bind _returnvalue_2 (Game|SpawnActorfromClass "/Game/Core/Player/BP_Cannonball.BP_Cannonball_C" (Math|Transform|MakeTransform _returnvalue) "Undefined" "MultiplyWithRoot" 0 0))
      (Physics|SetPhysicsLinearVelocity (Variables|/Game/Core/Player/BP_Cannonball.BP_Cannonball_C|GetStaticMesh _returnvalue_2) _outlaunchvelocity false "None"))))

(event EventBeginPlay
  (Utilities|FlowControl|Delay 0.0)
  (bind _asbp_game_mode (Utilities|Casting|CastToBP_GameMode (Game|GetGameMode)))
  (EventDispatchers|BindEventtoOnFinishMoving _asbp_game_mode (delegate Custom|FireCannon)))

(fn ConstructionScript)